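; Destroyed wreck Blueprint for the Z8J vehicle, with glass explosion and flame particle effects.
; Its construction script adds three glass explosion components and two flame components to ParticleSystemComponentArray.
; The script only registers the effects and contains no logic to trigger them.
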(fn ConstructionScript
  (bind _particlesystemcomponentarray (Variables|Default|GetParticleSystemComponentArray))
  (Utilities|Array|Add _particlesystemcomponentarray (Variables|Default|GetGlassExp))
  (Utilities|Array|Add _particlesystemcomponentarray (Variables|Default|GetGlassExp2))
  (Utilities|Array|Add _particlesystemcomponentarray (Variables|Default|GetGlassExp3))
  (Utilities|Array|Add _particlesystemcomponentarray (Variables|Default|GetFlame))
  (Utilities|Array|Add _particlesystemcomponentarray (Variables|Default|GetFlame2)))