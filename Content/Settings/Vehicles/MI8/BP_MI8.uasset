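; MI8 helicopter vehicle Blueprint that handles cockpit displays and the engine start-up and shutdown effects.
; Activation timelines drive readiness and material emissive, while remote instances reveal or hide screens, camera and lights.
; Enabling UI initializes the cockpit widgets; disabling collapses them so they stop ticking.
; Widget render targets and a camera render target feed dynamic materials on screen planes, retrying until the main targets are valid.
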(event Custom|ActivationSequence
  ;[0 0 0] flying
  (Utilities|FlowControl|Sequence
    (:then_0
      (Variables|Default|SetReadyToFly false)
      (bind _progress (Timeline|Timeline_0_0 PlayFromStart)
        (:Update
          (Class|SQHelicopterInstruments|SetActivationProgress _progress)
          (Utilities|FlowControl|DoOnce false
            (:Completed
              (Utilities|FlowControl|Sequence
                (:then_0
                  (Networking|SwitchHasAuthority
                    (:Remote
                      (Utilities|FlowControl|Delay 4.0)
                      (Rendering|SetVisibility (Variables|Default|GetEngineStats2) true false)
                      (Utilities|FlowControl|Delay 2.0)
                      (Rendering|SetVisibility (Variables|Default|GetDirectionScreen) true false))))
                (:then_1
                  (bind _lightintensity (Timeline|Timeline_1_0 Play)
                    (:Update
                      (Rendering|Material|SetScalarParameterValue (Variables|Default|GetMI8_Mat) "EmissiveMult" _lightintensity :!class /Script/Engine.MaterialInstanceDynamic))))))))
        (:Finished
          (Variables|Default|SetReadyToFly true)
          (Rendering|Components|Light|SetLightColor (Variables|Default|GetPointLight_0) "(R=0.000000,G=1.000000,B=0.635294,A=1.000000)" true))))
    (:then_1
      (Utilities|FlowControl|DoOnce false) ; enters at Reset
    )))

(event Custom|DeactivationSequence
  ;[0 0 0] flying
  (Utilities|FlowControl|DoOnce false
    (:Completed
      (Variables|Default|SetReadyToFly false)
      (Networking|SwitchHasAuthority
        (:Remote
          (Rendering|Components|Light|SetLightColor (Variables|Default|GetPointLight_0) "(R=1.000000,G=0.000000,B=0.000000,A=1.000000)" true)
          (Rendering|SetVisibility (Variables|Default|GetEngineStats2) false false)
          (Utilities|FlowControl|Sequence
            (:then_0
              (Utilities|FlowControl|DoOnce false) ; enters at Reset
            )
            (:then_1
              (bind _lightintensity (Timeline|Timeline_1_0 Stop)
                (:Update
                  (Rendering|Material|SetScalarParameterValue (Variables|Default|GetMI8_Mat) "EmissiveMult" _lightintensity :!class /Script/Engine.MaterialInstanceDynamic))))))))))

(event EventBeginPlay
  ;[1 1 1] BeginPlay
  (|CallParentFunction)
  (CallFunction|SetHelicopterWidgetsVisibility "Collapsed") ; collapsed = widgets cannot tick
  (Networking|CanExecuteCosmeticEvents
    (:True
      (bind _asw_helicopter_mini_map (Utilities|Casting|CastToW_Helicopter_MiniMap (UserInterface|GetUserWidgetObject (Variables|Default|GetMapDisplay))))
      (Default|InitializeMap _asw_helicopter_mini_map self))))

(event EventSetUIEnabled
  (params (Enable%20UI :type Boolean))
  (Networking|CanExecuteCosmeticEvents
    (:True
      (CallFunction|ManageHelicopterWidgets Enable%20UI)
      (bind _all_valid_ (CallFunction|SetHelicopterWidgetMaterials :!label _label))
      (if (not _all_valid_)
        (Utilities|FlowControl|Delay 0.4)
        (goto _label)))))

(fn ConstructionScript
  (bind _mi8matindex (Variables|Default|GetMi8MatIndex))
  (|CallParentFunction)
  (bind _returnvalue (Rendering|Material|CreateDynamicMaterialInstance (Variables|Default|GetVehicleMesh) _mi8matindex (Variables|Default|GetVehicleMesh_Material) "None" :!class /Script/Engine.PrimitiveComponent))
  (bind _output_get (Variables|Default|SetMI8_Mat _returnvalue))
  (Rendering|Material|SetMaterial (Variables|Default|GetVehicleMesh) _mi8matindex _output_get))

(fn GetUITint
  (return "(R=1.000000,G=0.983686,B=0.215000,A=1.000000)"))

(fn ManageHelicopterWidgets
  (params (Enabled :type Boolean))
  (bind _self self)
  (bind _self_2 self)
  (if Enabled
    (Utilities|FlowControl|Sequence
      (:then_0
        (bind _asw_mi8_main_display (Utilities|Casting|CastToW_MI8_MainDisplay (UserInterface|GetUserWidgetObject (Variables|Default|GetMainDisplay))))
        (Default|SetOwningVehicle _asw_mi8_main_display self)
        (Default|ManageUpdate _asw_mi8_main_display true)
        (bind _asw_mi8_main_display_2 (Utilities|Casting|CastToW_MI8_MainDisplay (UserInterface|GetUserWidgetObject (Variables|Default|GetCopilotDisplay))))
        (Default|SetOwningVehicle _asw_mi8_main_display_2 self)
        (Default|ManageUpdate _asw_mi8_main_display_2 true)
        (bind _asw_mi8_compass_display (Utilities|Casting|CastToW_MI8_CompassDisplay (UserInterface|GetUserWidgetObject (Variables|Default|GetCompass))))
        (Default|InitializeCompass _asw_mi8_compass_display self)
        (bind _asw_mi8_engine_stats (Utilities|Casting|CastToW_MI8_EngineStats (UserInterface|GetUserWidgetObject (Variables|Default|GetEngineStats))))
        (Default|InitializeDisplay _asw_mi8_engine_stats _self_2 (Variables|Default|GetEngine) _self_2)
        (bind _asw_mi8_engine_stats_2 (Utilities|Casting|CastToW_MI8_EngineStats (UserInterface|GetUserWidgetObject (Variables|Default|GetEngineStats2))))
        (Default|InitializeDisplay _asw_mi8_engine_stats_2 _self (Variables|Default|GetEngine) _self)
        (bind _asw_helicopter_direction (Utilities|Casting|CastToW_HelicopterDirection (UserInterface|GetUserWidgetObject (Variables|Default|GetDirectionScreen))))
        (Default|InitializeScreen _asw_helicopter_direction self))
      (:then_1
        (CallFunction|SetHelicopterWidgetsVisibility "HitTestInvisible")))
    (else
      (CallFunction|SetHelicopterWidgetsVisibility "Collapsed")
      (Utilities|FlowControl|Sequence
        (:then_0
          (bind _asw_mi8_main_display_3 (Utilities|Casting|CastToW_MI8_MainDisplay (UserInterface|GetUserWidgetObject (Variables|Default|GetMainDisplay))))
          (Default|ManageUpdate _asw_mi8_main_display_3 false))
        (:then_1
          (bind _asw_mi8_main_display_4 (Utilities|Casting|CastToW_MI8_MainDisplay (UserInterface|GetUserWidgetObject (Variables|Default|GetCopilotDisplay))))
          (Default|ManageUpdate _asw_mi8_main_display_4 false))))))

(fn SetHelicopterWidgetsVisibility
  (params (InVisibility :type ESlateVisibility%20Enum :default "Visible"))
  (Widget|SetVisibility (UserInterface|GetUserWidgetObject (Variables|Default|GetCopilotDisplay)) InVisibility))

(fn SetHelicopterWidgetMaterials
  (bind _screenmat (Variables|Default|GetScreenMat))
  (bind _maindisplay (Variables|Default|GetMainDisplay))
  (bind _compass (Variables|Default|GetCompass))
  (bind _mapdisplay (Variables|Default|GetMapDisplay))
  (bind _enginestats (Variables|Default|GetEngineStats))
  (bind _returnvalue (Class|WidgetComponent|GetRenderTarget _maindisplay))
  (bind _returnvalue_2 (Class|WidgetComponent|GetRenderTarget _compass))
  (bind _returnvalue_3 (Class|WidgetComponent|GetRenderTarget _enginestats))
  (bind _returnvalue_4 (Class|WidgetComponent|GetRenderTarget _mapdisplay))
  (Rendering|SetVisibility (Variables|Default|GetMainDisplay) true false)
  ;[1 1 1] Project widgets to screen planes
  (Class|WidgetComponent|RequestRedraw (Variables|Default|GetEngineStats))
  (bind _returnvalue_5 (Rendering|Material|CreateDynamicMaterialInstance (Variables|Default|GetMain%20Plane) 0 _screenmat "None" :!class /Script/Engine.PrimitiveComponent))
  (Rendering|Material|SetTextureParameterValue _returnvalue_5 "widgettexture" _returnvalue)
  (bind _returnvalue_6 (Rendering|Material|CreateDynamicMaterialInstance (Variables|Default|GetCopilot%20Plane) 0 _screenmat "None" :!class /Script/Engine.PrimitiveComponent))
  (Rendering|Material|SetTextureParameterValue _returnvalue_6 "widgettexture" _returnvalue)
  (bind _returnvalue_7 (Rendering|Material|CreateDynamicMaterialInstance (Variables|Default|GetCompass%20Plane) 0 _screenmat "None" :!class /Script/Engine.PrimitiveComponent))
  (Rendering|Material|SetTextureParameterValue _returnvalue_7 "widgettexture" _returnvalue_2)
  (bind _returnvalue_8 (Rendering|Material|CreateDynamicMaterialInstance (Variables|Default|GetMap%20Plane) 0 _screenmat "None" :!class /Script/Engine.PrimitiveComponent))
  (Rendering|Material|SetTextureParameterValue _returnvalue_8 "widgettexture" _returnvalue_4)
  (bind _returnvalue_9 (Rendering|Material|CreateDynamicMaterialInstance (Variables|Default|GetEngine%20Stats%20Plane) 0 _screenmat "None" :!class /Script/Engine.PrimitiveComponent))
  (Rendering|Material|SetTextureParameterValue _returnvalue_9 "widgettexture" _returnvalue_3)
  (bind _returnvalue_10 (Rendering|Material|CreateDynamicMaterialInstance (Variables|Default|GetEngine%20Stats%20Plane%202) 0 _screenmat "None" :!class /Script/Engine.PrimitiveComponent))
  (Rendering|Material|SetTextureParameterValue _returnvalue_10 "widgettexture" _returnvalue_3)
  (bind _returnvalue_11 (Rendering|Material|CreateDynamicMaterialInstance (Variables|Default|GetCamera%20Plane) 0 _screenmat "None" :!class /Script/Engine.PrimitiveComponent))
  (Rendering|Material|SetTextureParameterValue _returnvalue_11 "widgettexture" "/Game/Vehicles/UH60M/Textures/RT_UH60MCamera.RT_UH60MCamera")
  (bind _returnvalue_12 (Rendering|Material|CreateDynamicMaterialInstance (Variables|Default|GetDirection%20Plane) 0 _screenmat "None" :!class /Script/Engine.PrimitiveComponent))
  (Rendering|Material|SetTextureParameterValue _returnvalue_12 "widgettexture" (Class|WidgetComponent|GetRenderTarget (Variables|Default|GetDirectionDisplay)))
  (return (and (and (and (Utilities|IsValid _returnvalue) (Utilities|IsValid _returnvalue_2)) (Utilities|IsValid _returnvalue_4)) (Utilities|IsValid (Class|WidgetComponent|GetRenderTarget _enginestats)))))