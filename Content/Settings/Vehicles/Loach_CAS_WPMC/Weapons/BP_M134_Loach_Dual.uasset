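; Dual M134 minigun weapon for the Loach CAS helicopter, alternating fire between barrel sockets.
; Each shot sets the current barrel from rounds spent modulo socket count; the spawn transform uses the current barrel, the socket name the previous one.
; On top of the parent's effects, it spawns right-gun muzzle and shell-ejection emitters once, then toggles their IsPlaying parameter to start and stop looping.
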(event EventBlueprintonFire
  (params (Origin :type Vector%20%28by%20ref%29 :default "0, 0, 0"))
  (|CallParentFunction Origin)
  (CallFunction|UpdateCurrentBarrel))

(event EventStopFiringParticleEffects
  ;[0 0 0] Stop Looping Particles
  (|CallParentFunction)
  (for _array_element (Utilities|Array|MakeArray (Variables|Default|GetRightMuzzleParticle) (Variables|Default|GetRightShellEjectionParticle))
    (Utilities|IsValid _array_element
      (:Is%20Valid
        (Effects|Components|ParticleSystem|SetFloatParameter _array_element "IsPlaying" 0.0)))))

(event EventPlayFiringParticleEffects
  (params (InOrigin :type Vector%20%28by%20ref%29 :default "0, 0, 0"))
  (bind _returnvalue (Class|SQEquipableItem|IsFirstPersonViewTarget))
  (bind _mesh1p (Variables|Default|GetMesh1P))
  (bind _mesh3p (Variables|Default|GetMesh3P))
  (bind _weaponeffects (Variables|Default|GetWeaponEffects))
  (bind _returnvalue_2 (select _returnvalue _mesh1p _mesh3p))
  (|CallParentFunction InOrigin)
  (Networking|CanExecuteCosmeticEvents
    (:True
      (Utilities|FlowControl|Sequence
        (:then_0
          ;[0 0 0] Spawn Right Minigun (Once)
          (Networking|CanExecuteCosmeticEvents
            (:True
              (Utilities|IsValid (Variables|Default|GetRightMuzzleParticle)
                (:Is%20Valid
                  _)
                (:Is%20Not%20Valid
                  (bind _returnvalue_3 (Effects|SpawnEmitterAttached (select _returnvalue (.muzzleflasheffect3p _weaponeffects) (.muzzleflasheffect1p _weaponeffects)) _returnvalue_2 "M134_Muzzle_R" "0, 0, 0" "0, 0, 0" "1.000000,1.000000,1.000000" "SnapToTargetIncludingScale"))
                  (Variables|Default|SetRightMuzzleParticle _returnvalue_3)))
              (Utilities|IsValid (Variables|Default|GetRightShellEjectionParticle)
                (:Is%20Not%20Valid
                  (bind _returnvalue_4 (Effects|SpawnEmitterAttached (select _returnvalue (.shellejection3p _weaponeffects) (.shellejection1p _weaponeffects)) _returnvalue_2 "M134_ShellEjection_R" "0, 0, 0" "0, 0, 0" "1.000000,1.000000,1.000000" "SnapToTargetIncludingScale"))
                  (Variables|Default|SetRightShellEjectionParticle _returnvalue_4))))))
        (:then_1
          ;[0 0 0] Start Looping Particles
          (Utilities|IsValid (Variables|Default|GetRightMuzzleParticle)
            (:Is%20Valid
              (Effects|Components|ParticleSystem|SetFloatParameter (Variables|Default|GetRightMuzzleParticle) "IsPlaying" 1.0)
              (if (and (Utilities|IsValid (Variables|Default|GetRightShellEjectionParticle)) (Class|SQWeaponEffects|CanPlayShellEjections))
                (Effects|Components|ParticleSystem|SetFloatParameter (Variables|Default|GetRightShellEjectionParticle) "IsPlaying" 1.0)))))))))

(fn ConstructionScript
  (|CallParentFunction))

(fn UpdateCurrentBarrel
  (bind _magazines (Variables|Default|GetMagazines))
  (bind _output (Utilities|Array|Get(acopy) _magazines))
  (bind (_defaultroundspermag _remainingrounds) (Utilities|Struct|BreakSQMagazineData _output))
  (Variables|Default|SetLastBarrel (Variables|Default|GetCurrentBarrel))
  (bind _output_get (LocalVariables|SetNumBarrels (Utilities|Array|Length (Variables|Default|GetBarrelSockets))))
  (if (> _output_get 1)
    (Variables|Default|SetCurrentBarrel (Math|Integer|%(Integer) (- _defaultroundspermag _remainingrounds) (LocalVariables|GetNumBarrels)))
    (else
      (Variables|Default|SetCurrentBarrel 0))))

(fn GetProjectileSpawnTransform
  (return (Transformation|GetSocketTransform (Variables|Default|GetMesh1P) (Utilities|Array|Get(acopy) (Variables|Default|GetBarrelSockets) (Variables|Default|GetCurrentBarrel)) "RTS_World")))

(fn GetProjectileSpawnSocketName
  (return (Utilities|Array|Get(acopy) (Variables|Default|GetBarrelSockets) (Variables|Default|GetLastBarrel))))