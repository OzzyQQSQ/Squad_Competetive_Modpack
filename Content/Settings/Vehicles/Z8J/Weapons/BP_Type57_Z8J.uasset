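; Type 57 weapon Blueprint for the Z8J vehicle, handling alternating-pod firing and staged overheat feedback.
; Each shot teleports the first- and third-person meshes between two pod Y offsets, then triggers a blast when cosmetic events are allowed.
; Temperature triggers set the overheat flag and switch between three stages of DShK particles and HMG looping sounds.
; Effects are spawned lazily on the viewed mesh, then reused through activation and audio fades.
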(event EventBlueprintonFire
  (params (Origin :type Vector%20%28by%20ref%29 :default "0, 0, 0"))
  (|CallParentFunction Origin)
  (if (< (Variables|Default|GetCurrentShot) 2)
    _
    (else
      (Variables|Default|SetCurrentShot 0)))
  (Transformation|SetRelativeLocation (Variables|Default|GetMesh1P) (Math|Vector|MakeVector 0.0 (Utilities|Array|Get(acopy) (Variables|Default|GetPodLocations) (Variables|Default|GetCurrentShot)) 0.0) false true)
  (Math|Integer|IncrementInt (Variables|Default|GetCurrentShot)
    (:%20%20
      (Networking|CanExecuteCosmeticEvents
        (:True
          (Class|SQBlastComponent|FireBlast (Variables|Default|GetSQBlast)))))))

(fn ConstructionScript)