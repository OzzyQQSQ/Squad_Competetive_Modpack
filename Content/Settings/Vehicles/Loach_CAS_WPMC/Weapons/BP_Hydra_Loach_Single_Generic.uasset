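; Single-fire Hydra weapon Blueprint for the Loach CAS helicopter, extending its parent's fire event with a cosmetic-only SQBlast.
; Also defines three-stage overheat macros that choose particles and looping sounds by triggering temperature and flag overheating at shutdown temperature.
; Effects borrow DSHK/HMG assets, spawn once on the first- or third-person mesh, then get reused through activation and fades.
; The event graph shown never calls the overheat logic.
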(event EventBlueprintonFire
  (params (Origin :type Vector%20%28by%20ref%29 :default "0, 0, 0"))
  (|CallParentFunction Origin)
  (Networking|CanExecuteCosmeticEvents
    (:True
      (Class|SQBlastComponent|FireBlast (Variables|Default|GetSQBlast)))))

(fn ConstructionScript)