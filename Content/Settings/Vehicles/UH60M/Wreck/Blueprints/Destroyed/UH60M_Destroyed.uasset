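; UH60M_Destroyed is the destroyed wreck Blueprint for the UH-60M helicopter, carrying particle effects that include a glass explosion and fire.
; Its construction script adds five particle system components to ParticleSystemComponentArray: GlassExp, three generically named systems and Fire.
; The graph only fills that array and contains no logic that activates or otherwise uses the effects.
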(fn ConstructionScript
  (bind _particlesystemcomponentarray (Variables|Default|GetParticleSystemComponentArray))
  (Utilities|Array|Add _particlesystemcomponentarray (Variables|Default|GetGlassExp))
  (Utilities|Array|Add _particlesystemcomponentarray (Variables|Default|GetParticleSystem))
  (Utilities|Array|Add _particlesystemcomponentarray (Variables|Default|GetParticleSystem1))
  (Utilities|Array|Add _particlesystemcomponentarray (Variables|Default|GetParticleSystem2))
  (Utilities|Array|Add _particlesystemcomponentarray (Variables|Default|GetFire)))