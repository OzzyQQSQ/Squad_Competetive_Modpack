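; Z-8J vehicle weapon Blueprint for the Type 23 gun, handling firing feedback and barrel overheating.
; Each shot shifts the 1P and 3P meshes between two pod positions in alternation, adds heat, plays the fire animation and shakes the camera.
; Temperature threshold events set the overheated flag and drive three stages of lazily spawned, reused particles and looping sounds, faded or deactivated outside their stage.
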(event OnTemperatureIncrementEvent(SQTemperature)
  (params (TriggeringComponent :type SQ%20Temperature%20Component%20Object%20Reference) (TriggeringTemp :type Float%20%28single-precision%29) (bIsLowerTrigger :type Boolean))
  (Utilities|FlowControl|Sequence
    (:then_0
      (Utilities|SetOverheatVariable bIsLowerTrigger TriggeringTemp))
    (:then_1
      (Utilities|SetupOverheatEffect bIsLowerTrigger TriggeringTemp))))

(event EventBlueprintonFire
  (params (Origin :type Vector%20%28by%20ref%29 :default "0, 0, 0"))
  (|CallParentFunction Origin)
  (if (< (Variables|Default|GetCurrentShot) 2)
    _
    (else
      (Variables|Default|SetCurrentShot 0)))
  (Transformation|SetRelativeLocation (Variables|Default|GetMesh1P) (Math|Vector|MakeVector 0.0 (Utilities|Array|Get(acopy) (Variables|Default|GetPodLocations) (Variables|Default|GetCurrentShot)) 0.0) false true)
  (Class|SQTemperatureComponent|AdjustTemperature (Variables|Temperature|GetSQTemperature) 1.0 0)
  (Class|SQVehicleWeapon|PlayVehicleWeaponAnimations 0 (Variables|Default|GetWeaponFireAnim) 0 0.0)
  (Math|Integer|IncrementInt (Variables|Default|GetCurrentShot)
    (:%20%20
      (Camera|PlayWorldCameraShake (Variables|Default|GetCameraShakeOnFire) (Transformation|GetSocketLocation (select (Class|SQEquipableItem|IsFirstPersonViewTarget) (Variables|Default|GetMesh1P) (Variables|Default|GetMesh3P)) "ShellEjection") 0.0 1e+02 1.0 true))))

(fn ConstructionScript)