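; Vehicle Blueprint for the USMC woodland utility M939 truck, handling visual wheel loss and restoration.
; Drivetrain destroyed and repaired events filter for SQVehicleWheel components and pass the bone name to UpdateDamageWheelVisual.
; That function hides or restores each of the six wheels by setting its scale variable on the ABP_M939Truck anim instance to zero or one.
; The DoEffects input is currently unused.
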(event EventDrivetrainComponentDestroyed
  (params (DriveTrainComponent :type SQ%20Drive%20Train%20Component%20Object%20Reference))
  ;[1 1 1] Wheel Bindings
  (bind _assqvehicle_wheel (Utilities|Casting|CastToSQVehicleWheel DriveTrainComponent))
  (CallFunction|UpdateDamageWheelVisual (Class|SQVehicleWheel|GetBoneName _assqvehicle_wheel) true _assqvehicle_wheel true))

(event EventDrivetrainComponentRepaired
  (params (DriveTrainComponent :type SQ%20Drive%20Train%20Component%20Object%20Reference))
  ;[1 1 1] Wheel Bindings
  (bind _assqvehicle_wheel (Utilities|Casting|CastToSQVehicleWheel DriveTrainComponent))
  (CallFunction|UpdateDamageWheelVisual (Class|SQVehicleWheel|GetBoneName _assqvehicle_wheel) false _assqvehicle_wheel false))

(fn ConstructionScript)

(fn UpdateDamageWheelVisual
  (params (Bone :type Name) (Destroyed :type Boolean) (Wheel :type SQ%20Vehicle%20Wheel%20Object%20Reference) (Do%20Effects :type Boolean))
  ;[1 1 1] Set Wheel Scale to 0
  (LocalVariables|SetL%20Scale (select Destroyed "0, 0, 0" "1.000000,1.000000,1.000000"))
  (bind _asabp_m939truck (Utilities|Casting|CastToABP_M939Truck (Components|SkeletalMesh|GetAnimInstance (Variables|Default|GetVehicleMesh))))
  (switch name Bone
    (:wheel_L1
      (Variables|/Game/Vehicles/US_Util_Truck/Meshes/ABP_M939Truck.ABP_M939Truck_C|SetWheel%20L1%20Scale _asabp_m939truck (LocalVariables|GetL%20Scale)))
    (:wheel_L2
      (Variables|/Game/Vehicles/US_Util_Truck/Meshes/ABP_M939Truck.ABP_M939Truck_C|SetWheel%20L2%20Scale _asabp_m939truck (LocalVariables|GetL%20Scale)))
    (:wheel_L3
      (Variables|/Game/Vehicles/US_Util_Truck/Meshes/ABP_M939Truck.ABP_M939Truck_C|SetWheel%20L3%20Scale _asabp_m939truck (LocalVariables|GetL%20Scale)))
    (:wheel_R1
      (Variables|/Game/Vehicles/US_Util_Truck/Meshes/ABP_M939Truck.ABP_M939Truck_C|SetWheel%20R1%20Scale _asabp_m939truck (LocalVariables|GetL%20Scale)))
    (:wheel_R2
      (Variables|/Game/Vehicles/US_Util_Truck/Meshes/ABP_M939Truck.ABP_M939Truck_C|SetWheel%20R2%20Scale _asabp_m939truck (LocalVariables|GetL%20Scale)))
    (:wheel_R3
      (Variables|/Game/Vehicles/US_Util_Truck/Meshes/ABP_M939Truck.ABP_M939Truck_C|SetWheel%20R3%20Scale _asabp_m939truck (LocalVariables|GetL%20Scale)))))