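; Crashed UH-60M helicopter wreck actor, built from mesh pieces, particle systems and radial force components.
; When the front trail emitter spawns particles, it plays an attached burning loop sound and stops it after the emitter time.
; The construction script gathers the particle systems into an array, which nothing here reads.
; An unconnected chain, which never runs, would fire a radial impulse, then destroy wreck pieces after staggered random delays.
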(event OnParticleSpawn(FrontTrail)
  (params (EventName :type Name :default "None") (EmitterTime :type Float%20%28single-precision%29) (Location :type Vector :default "0, 0, 0") (Velocity :type Vector :default "0, 0, 0"))
  (bind _returnvalue (Audio|SpawnSoundAttached "/Game/Audio/Vehicles/Damage/ChopperDamage/Burning/Chopper_Burning_Loop_01_Cue.Chopper_Burning_Loop_01_Cue" 0 "None" "0, 0, 0" "0, 0, 0" "KeepRelativeOffset" false 1.0 1.0 0.0 0 0))
  (Audio|Components|Audio|Play _returnvalue 0.0)
  (Utilities|FlowControl|Delay EmitterTime)
  (Audio|Components|Audio|Stop _returnvalue))

(event EventBeginPlay)

(fn ConstructionScript
  (bind _particlesystemcomponentarray (Variables|Default|GetParticleSystemComponentArray))
  (Utilities|Array|Add _particlesystemcomponentarray (Variables|Default|GetFrontTrail))
  (Utilities|Array|Add _particlesystemcomponentarray (Variables|Default|GetTrail))
  (Utilities|Array|Add _particlesystemcomponentarray (Variables|Default|GetParticleSystem))
  (Utilities|Array|Add _particlesystemcomponentarray (Variables|Default|GetParticleSystem1))
  (Utilities|Array|Add _particlesystemcomponentarray (Variables|Default|GetParticleSystem2))
  (Utilities|Array|Add _particlesystemcomponentarray (Variables|Default|GetParticleSystem3)))