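; Crash wreck actor for the Z8J helicopter, with breakaway debris, particle effects and burning audio.
; On BeginPlay a radial force fires an impulse, both force components are removed shortly after, then selected mesh pieces are destroyed at independently randomized delays.
; A particle spawn event on one emitter plays an attached burning loop, stopped after a delay equal to its EmitterTime.
; The construction script collects the particle systems into an array.
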(event OnParticleSpawn(ParticleSystem4)
  (params (EventName :type Name :default "None") (EmitterTime :type Float%20%28single-precision%29) (Location :type Vector :default "0, 0, 0") (Velocity :type Vector :default "0, 0, 0"))
  (bind _returnvalue (Audio|SpawnSoundAttached "/Game/Audio/Vehicles/Damage/ChopperDamage/Burning/Chopper_Burning_Loop_01_Cue.Chopper_Burning_Loop_01_Cue" 0 "None" "0, 0, 0" "0, 0, 0" "KeepRelativeOffset" false 1.0 1.0 0.0 0 0))
  (Audio|Components|Audio|Play _returnvalue 0.0)
  (Utilities|FlowControl|Delay EmitterTime)
  (Audio|Components|Audio|Stop _returnvalue))

(event EventBeginPlay
  (bind _returnvalue (Math|Random|RandomFloatinRange 4e+01 45.0))
  (Class|RadialForceComponent|FireImpulse (Variables|Default|GetRadialForce))
  (Utilities|FlowControl|Delay 0.5)
  (Components|DestroyComponent (Variables|Default|GetRadialForce))
  (Utilities|FlowControl|Sequence
    (:then_0
      (Utilities|FlowControl|Delay _returnvalue)
      (Components|DestroyComponent (Variables|Default|GetLargeMesh6)))
    (:then_1
      (Utilities|FlowControl|Delay _returnvalue)
      (Components|DestroyComponent (Variables|Default|GetLargeMesh7)))
    (:then_2
      (Utilities|FlowControl|Delay _returnvalue)
      (Components|DestroyComponent (Variables|Default|GetLargeMesh4)))
    (:then_3
      (Utilities|FlowControl|Delay _returnvalue)
      (Components|DestroyComponent (Variables|Default|GetStaticMesh5)))
    (:then_4
      (Utilities|FlowControl|Delay _returnvalue)
      (Components|DestroyComponent (Variables|Default|GetStaticMesh7)))
    (:then_5
      (Utilities|FlowControl|Delay _returnvalue)
      (Components|DestroyComponent (Variables|Default|GetLargeMesh5)))
    (:then_6
      (Utilities|FlowControl|Delay _returnvalue)
      (Components|DestroyComponent (Variables|Default|GetLargeMesh2)))
    (:then_7
      (Utilities|FlowControl|Delay _returnvalue)
      (Components|DestroyComponent (Variables|Default|GetStaticMesh4)))))

(fn ConstructionScript
  (bind _particlesystemcomponentarray (Variables|Default|GetParticleSystemComponentArray))
  (Utilities|Array|Add _particlesystemcomponentarray (Variables|Default|GetParticleSystem))
  (Utilities|Array|Add _particlesystemcomponentarray (Variables|Default|GetParticleSystem1))
  (Utilities|Array|Add _particlesystemcomponentarray (Variables|Default|GetParticleSystem2))
  (Utilities|Array|Add _particlesystemcomponentarray (Variables|Default|GetParticleSystem3))
  (Utilities|Array|Add _particlesystemcomponentarray (Variables|Default|GetParticleSystem4))
  (Utilities|Array|Add _particlesystemcomponentarray (Variables|Default|GetParticleSystem5)))