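; Commander scope turret for the Z8J vehicle, providing a rotatable, zoomable first-person sight.
; The construction script registers TurretMovement, yawing the scene root and pitching GunAttachPoint, which also anchors views and weapon, while the soldier attaches to the vehicle mesh.
; Fire input drives the vehicle inventory's current weapon.
; Zoom uses a timeline to blend FOV toward the user's setting divided by the zoom level, and reset restores the first-person camera.
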(event EventResetZoom
  ;[0 0.685 0.1713] ZoomEvents
  (Camera|SetFieldOfView (Variables|Default|GetFirstPersonCamera) (/ (Variables|/Script/Squad.SQGameUserSettings|GetFOV (Class|SQBlueprintLibrary|GetSquadGameUserSettings)) (Utilities|Array|Get(acopy) (Variables|Default|GetZoomLevels))))
  (Components|Activation|SetActive (Variables|Default|GetCamera) false false)
  (Components|Activation|SetActive (Variables|Default|GetFirstPersonCamera) true false)
  (Variables|Default|SetCurrentZoom 0))

(event EventOnVehicleZoom
  (bind _firstpersoncamera (Variables|Default|GetFirstPersonCamera))
  ;[0 0.685 0.1713] ZoomEvents
  (bind _lerp (Timeline|Timeline_0 PlayFromStart)
    (:Update
      (Camera|SetFieldOfView _firstpersoncamera (Math|Float|Lerp (Variables|/Script/Engine.CameraComponent|GetFieldOfView _firstpersoncamera) (/ (Variables|/Script/Squad.SQGameUserSettings|GetFOV (Class|SQBlueprintLibrary|GetSquadGameUserSettings)) (Utilities|Array|Get(acopy) (Variables|Default|GetZoomLevels) (Variables|Default|GetCurrentZoom))) _lerp)))))

(event EventBeginPlay
  (Components|Activation|SetActive (Variables|Default|GetFirstPersonCamera) true false)
  (Variables|/Script/Squad.SQMovementComponentBase|SetMaxSpeed (Variables|Default|GetTurretMovement) (select true 6e+01 0.0)))

(event Input|ActionEvents|InputActionFire
  (params (Key :type Key%20Structure))
  (bind _returnvalue (Class|SQVehicleSeat|GetVehicleInventory))
  (bind _currentweapon (Variables|/Script/Squad.SQPawnInventoryComponent|GetCurrentWeapon _returnvalue))
  (:Pressed
    (Class|SQEquipableItem|BeginUse _currentweapon))
  (:Released
    (Class|SQEquipableItem|EndUse _currentweapon)))

(fn ConstructionScript
  (bind _turretmovement (Variables|Default|GetTurretMovement))
  (bind _defaultsceneroot (Variables|Default|GetDefaultSceneRoot))
  (Utilities|FlowControl|Sequence
    (:then_0
      (Variables|/Script/Squad.SQVelocityRotatingMovementComponent|SetUpdatedComponent _turretmovement _defaultsceneroot)
      (Variables|/Script/Squad.SQTurretMovementComponent|SetUpdatedYawComponent _turretmovement _defaultsceneroot)
      (Variables|/Script/Squad.SQVelocityRotatingMovementComponent|SetUpdatedComponent _turretmovement (Variables|Default|GetGunAttachPoint))
      (Variables|/Script/Squad.SQTurretMovementComponent|SetUpdatedPitchComponent _turretmovement (Variables|Default|GetGunAttachPoint))
      (Variables|/Script/Squad.SQVelocityRotatingMovementComponent|SetHeadingParentComponent _turretmovement _turretmovement)
      (Class|SQMovementComponentManager|RegisterComponent (Variables|Default|GetMovementComponentManager) _turretmovement))))

(fn Get3PAttachComponent
  (return (Variables|Default|GetGunAttachPoint)))

(fn Get1PAttachComponent
  (return (Variables|Default|GetGunAttachPoint)))

(fn GetMasterPoseComponent
  (return 0))

(fn GetWeaponAttachComponent
  (return (Variables|Default|GetGunAttachPoint)))

(fn GetSoldierAttachComponent
  (return (Variables|/Script/Squad.SQVehicle|GetVehicleMesh (Class|SQVehicleSeat|GetVehicle))))

(fn GetTurretMovementComponent
  (return (Variables|Default|GetTurretMovement)))