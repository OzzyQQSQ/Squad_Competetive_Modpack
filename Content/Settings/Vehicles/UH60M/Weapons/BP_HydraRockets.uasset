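; Hydra rocket weapon for the UH60M helicopter, with graphs for three stages of overheat feedback and the overheated state.
; Setup Overheat Effect matches the triggering temperature to a stage, fading out the others' sounds and deactivating their particles after delays.
; Each stage lazily spawns and reuses DSHK particles and HMG sounds, attached to the first- or third-person mesh.
; Set Overheat Variable flags overheating at shutdown temperature unless it is a lower trigger.
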(fn ConstructionScript)