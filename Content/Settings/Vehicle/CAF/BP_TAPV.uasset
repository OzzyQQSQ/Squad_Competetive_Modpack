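; BP_TAPV is the Blueprint for the TAPV wheeled vehicle, handling the visual side of wheel damage.
; On a wheel damage update, it sets the matching scale variable on the mesh's TAPV_AnimBlueprint to zero when destroyed, or full size otherwise.
; Each of the four wheels is selected by bone, so destroyed wheels are hidden through the animation Blueprint rather than separate mesh components.
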(event EventBeginPlay
  (|CallParentFunction) ; This node is disabled and will not be called.\nDrag off pins to build functionality.
)

(event Collision|EventActorBeginOverlap
  (params (OtherActor :type Actor%20Object%20Reference)))

(event EventTick
  (params (DeltaSeconds :type Float%20%28single-precision%29)))

(event EventUpdateDamageWheelVisual
  (params (Bone :type Name :default "None") (Destroyed :type Boolean) (Wheel :type SQ%20Vehicle%20Wheel%20Object%20Reference) (Do%20Effects :type Boolean))
  ;[1 1 1] Set Wheel Scale to 0
  (Variables|Default|SetL%20Scale_0 (select Destroyed "0, 0, 0" "1.000000,1.000000,1.000000"))
  (bind _astapv_anim_blueprint (Utilities|Casting|CastToTAPV_AnimBlueprint (Components|SkeletalMesh|GetAnimInstance (Variables|Default|GetVehicleMesh))))
  (switch name Bone
    (:wheel_L1
      (Variables|/Game/Vehicles/TAPV/Meshes/TAPV_AnimBlueprint.TAPV_AnimBlueprint_C|SetWheel%20L1%20Scale _astapv_anim_blueprint (Variables|Default|GetL%20Scale_0)))
    (:wheel_L2
      (Variables|/Game/Vehicles/TAPV/Meshes/TAPV_AnimBlueprint.TAPV_AnimBlueprint_C|SetWheel%20L2%20Scale _astapv_anim_blueprint (Variables|Default|GetL%20Scale_0)))
    (:wheel_R1
      (Variables|/Game/Vehicles/TAPV/Meshes/TAPV_AnimBlueprint.TAPV_AnimBlueprint_C|SetWheel%20R1%20Scale _astapv_anim_blueprint (Variables|Default|GetL%20Scale_0)))
    (:wheel_R2
      (Variables|/Game/Vehicles/TAPV/Meshes/TAPV_AnimBlueprint.TAPV_AnimBlueprint_C|SetWheel%20R2%20Scale _astapv_anim_blueprint (Variables|Default|GetL%20Scale_0)))))

(fn ConstructionScript
  (|CallParentFunction))